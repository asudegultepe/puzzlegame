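; Game mode Blueprint for a puzzle game that shows the completion screen and carries debug hotkeys.
; BeginPlay moves the PC_PuzzlePlayerController actor to a fixed raised location.
; Space, C and T test piece spawning, completion checking and move counting, though the EnableInput node is unconnected.
; OnGameComplete creates WBP_GameComplete with the final time and move total and adds it to the viewport.
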(event `Key|SpaceBar`
  (params (Key :type "Key Structure"))
  (:`Pressed`
    (`|SpawnActorFromClass` "/Game/Blueprints/BP_PuzzlePiece.BP_PuzzlePiece_C" (`KismetMathLibrary.MakeTransform` (0.0 0.0 0.0)) "Undefined" "MultiplyWithRoot" null null)
    (`KismetSystemLibrary.PrintString` "piece spawn")))

(event `Key|C`
  (params (Key :type "Key Structure"))
  (:`Pressed`
    (bind _returnvalue (`self.CheckGameCompletion`))
    (if _returnvalue
      (`KismetSystemLibrary.PrintString` "game COMPLETED")
      (else
        (`KismetSystemLibrary.PrintString` "not completed")))))

(event `self.ReceiveBeginPlay`
  (`GameplayStatics.GetActorOfClass` "/Game/Blueprints/BP_PuzzlePawn.BP_PuzzlePawn_C")
  (bind _returnvalue (`GameplayStatics.GetActorOfClass` "/Game/Blueprints/PC_PuzzlePlayerController.PC_PuzzlePlayerController_C"))
  (`self.K2_SetActorLocation` _returnvalue (0.0 0.0 1000.0) false false))

(event `Key|T`
  (params (Key :type "Key Structure"))
  (:`Pressed`
    (`self.IncrementMoveCount`)
    (`KismetSystemLibrary.PrintString` "move count increased")))

(fn `OnGameComplete`
  (bind _returnvalue (`|CreateWidget` "/Game/Widgets/WBP_GameComplete.WBP_GameComplete_C" null (`self.GameTime`) (`self.TotalMoves`)))
  (`UserWidget.AddToViewport` _returnvalue 999))

(fn `UserConstructionScript`)