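; Player controller for a puzzle game that sets up the main UI, camera and input state at play start.
; BeginPlay, gated on a MainWidget validity check, adds WBP_MainWidget to the viewport, then moves BP_PuzzlePawn to a fixed elevated position.
; It then sets the pawn's CineCamera to auto-activate and ignores move and look input.
; OnPieceSelected only prints the piece name; UI-only input and FOV nodes are unwired.
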(event `self.ReceiveBeginPlay`
  (if (`KismetSystemLibrary.IsValid` (`self.MainWidget`))
    (bind _returnvalue (`|CreateWidget` "/Game/Widgets/WBP_MainWidget.WBP_MainWidget_C" null null))
    (bind _output_get (set `self.MainWidgetVar` _returnvalue))
    (`UserWidget.AddToViewport` _output_get 0)
    (`KismetSystemLibrary.PrintString` "main widget added to viewport")
    (bind _asbp_puzzle_pawn (cast `/Game/Blueprints/BP_PuzzlePawn` (`GameplayStatics.GetPlayerPawn` 0)))
    (`self.K2_SetActorLocation` _asbp_puzzle_pawn (0.0 0.0 1000.0) false false)
    (`ActorComponent.SetAutoActivate` (`/Game/Blueprints/BP_PuzzlePawn.CineCamera` _asbp_puzzle_pawn) true)
    (`self.SetIgnoreMoveInput` true)
    (`self.SetIgnoreLookInput` true)
    (else
      (`KismetSystemLibrary.PrintString` "main widget nor set" true true (struct :`R` 1.0 :`A` 1.0)))))

(event `self.OnPieceSelected`
  (params (Piece :type "PuzzlePiece Object Reference"))
  (`KismetSystemLibrary.PrintString` (`KismetSystemLibrary.GetDisplayName` Piece)))

(fn `UserConstructionScript`)